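; Actor component that turns its owner into a quest giver with a floating quest marker.
; BeginPlay builds a Quest object from QuestDataRef and adds a marker widget offset upward by the owner's bounds.
; Interact enables the quest with the player channel and HUD quest book, hiding the marker, or, once all objectives are complete, disables it and destroys marker and component.
; UpdateQuestMarker re-shows the marker with the QuestValid icon.
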(event `self.ReceiveBeginPlay`
  ;[1 1 1] Event BeginPlay
  (`|ExecutionSequence`
    (:`then_0`
      (`self.QuestDataRef`
        (:`then`
          (bind _returnvalue (`|GenericCreateObject` "/Script/DemoreelRPG.Quest"))
          (bind _output_get (set `self.MyQuest` _returnvalue))
          (`self.SetQuestData` _output_get))
        (:`else`)))
    (:`then_1`
      (`self.CreateQuestMarker`))))

(event `/Game/MyGame/Blueprints/Interfaces/BPI_Interactable.Interact`
  (params (`Player Channel` :type "PlayerChannels Object Reference"))
  ;[1 1 1] Interaction with the quest giver
  (if (not (`self.IsQuestEnable`))
    (`self.EnableQuest` `Player Channel`)
    (elif (`Quest.isAllObjectivesComplet` (`self.MyQuest`))
      (`self.DisableQuest`))))

(event `self.UpdateQuestMarker`
  ;[1 1 1] Update Quest Marker
  (`Image.SetBrush` (`/Game/MyGame/Tools/QuestTool/Components/WBP_QuestMark.Sprite` (`self.QuestMarkWidget`)) (make `SlateBrush` "Image" "NoTile" "NoMirror" (make `DeprecateSlateVector2D` 100.0 100.0) (struct) (struct :`SpecifiedColor` (struct :`R` 1.0 :`G` 1.0 :`B` 1.0 :`A` 1.0) :`ColorUseRule` "UseColor_Specified") (struct :`CornerRadii` (struct :`W` 1.0) :`Color` (struct :`SpecifiedColor` (struct) :`ColorUseRule` "UseColor_Specified") :`RoundingType` "HalfHeightRadius") "/Game/MyGame/Art/UI/QuestValid.QuestValid"))
  (`SceneComponent.SetVisibility` (`self.MyWidgetComponent`) true false))

(fn `CreateQuestMarker`
  (bind _returnvalue (`self.GetOwner`))
  (`|ExecutionSequence`
    (:`then_0`
      ;[1 1 1] Create the QuestMarker Widget
      (bind _returnvalue_2 (`|AddComponentByClass` :`self` _returnvalue :`Class` "/Script/UMG.WidgetComponent"))
      (set `self.MyWidgetComponent` _returnvalue_2)
      (bind _returnvalue_3 (`|CreateWidget` "/Game/MyGame/Tools/QuestTool/Components/WBP_QuestMark.WBP_QuestMark_C"))
      (bind _output_get (set `self.QuestMarkWidget` _returnvalue_3))
      (`WidgetComponent.SetWidget` _returnvalue_2 _output_get)
      (`PrimitiveComponent.SetMaterial` _returnvalue_2 0 "/Engine/EngineMaterials/Widget3DPassThroughTwoSided.Widget3DPassThroughTwoSided"))
    (:`then_1`
      ;[1 1 1] Place it at the top of the owner
      (bind (_center _boxextent) (`GameplayStatics.GetActorArrayBounds` (`|MakeArray` _returnvalue)))
      (`SceneComponent.K2_AddWorldOffset` (`self.MyWidgetComponent`) (`KismetMathLibrary.MakeVector` 0.0 0.0 (/ (.z _boxextent) 1.5)) false false))))

(fn `DisableQuest`
  (`Quest.DisableQuest` (`self.MyQuest`))
  (`self.RemoveWidgetComponent`)
  ;[1 1 1] Remove QuestGiverComponent from the actor
  (`self.K2_DestroyComponent`))

(fn `EnableQuest`
  (params (PlayerChannel :type "PlayerChannels Object Reference"))
  ;[1 1 1] Could replace this by a Quest Channel on the player
  (bind _asbp_hud (cast `/Game/MyGame/3C/_HUD/BP_HUD` (`PlayerController.GetHUD` (`GameplayStatics.GetPlayerController` 0))))
  ;[1 1 1] Enable Queset and hide QuestMarker Widget
  (`Quest.EnableQuest` (`self.MyQuest`) PlayerChannel (`/Game/MyGame/3C/_HUD/BP_HUD.BookQuestWidget` _asbp_hud) self)
  (set `self.IsQuestEnable` true)
  (`SceneComponent.SetVisibility` (`self.MyWidgetComponent`) false false))

(fn `RemoveWidgetComponent`
  (bind _mywidgetcomponent (`self.MyWidgetComponent`))
  (`WidgetComponent.SetWidget` _mywidgetcomponent null)
  (`self.K2_DestroyComponent` _mywidgetcomponent))

(fn `SetQuestData`
  (params (Quest :type "Quest Object Reference"))
  (bind _mydata (`Quest.myData` Quest))
  (bind _questdataref (`self.QuestDataRef`))
  (set `QuestData.objectives` (`QuestData.objectives` _questdataref) _mydata)
  (set `QuestData.questTitle` (`QuestData.questTitle` _questdataref) _mydata)
  (set `QuestData.questDescription` (`QuestData.questDescription` _questdataref) _mydata))