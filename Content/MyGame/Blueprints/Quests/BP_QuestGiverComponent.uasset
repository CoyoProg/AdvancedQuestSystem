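; BP_QuestGiverComponent is a quest giver component that hands out a single quest and closes it once its objectives are complete.
; It constructs the quest object from QuestRef at BeginPlay.
; The first Interact enables the quest, passing the player channel, the HUD's quest book widget and itself.
; Later interactions check completion; when all objectives are done, they disable the quest and destroy the component.
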(event `self.ReceiveBeginPlay`
  (bind _returnvalue (`|GenericCreateObject` (`self.QuestRef`)))
  (set `self.MyQuest` _returnvalue))

(event `/Game/MyGame/Blueprints/Interfaces/BPI_Interactable.Interact`
  (params (`Player Channel` :type "PlayerChannels Object Reference"))
  ;[1 1 1] Simulate new Quest Enable
  (if (not (`self.IsQuestEnable`))
    (bind _asbp_hud (cast `/Game/MyGame/3C/_HUD/BP_HUD` (`PlayerController.GetHUD` (`GameplayStatics.GetPlayerController` 0))))
    (`Quest.EnableQuest` (`self.MyQuest`) `Player Channel` (`/Game/MyGame/3C/_HUD/BP_HUD.BookQuestWidget` _asbp_hud) self)
    (set `self.IsQuestEnable` true)
    (elif (`Quest.isAllObjectivesComplet` (`self.MyQuest`))
      (`Quest.DisableQuest` (`self.MyQuest`))
      (`self.K2_DestroyComponent`))))