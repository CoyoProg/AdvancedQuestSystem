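; Test Blueprint that simulates enabling a new quest, exercising the quest system and quest book UI.
; On BeginPlay it constructs a quest from QuestRef, enables it with the player character's PlayerChannels, then adds it to the HUD's QuestBookWidget after a short delay.
; For debugging, Tick runs through a Delay to refresh that quest in the quest book every few seconds.
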(event `self.ReceiveBeginPlay`
  ;[1 1 1] Simulate new Quest Enable
  (`|ExecutionSequence`
    (:`then_0`
      (bind _returnvalue (`|GenericCreateObject` (`self.QuestRef`)))
      (set `self.MyQuest` _returnvalue))
    (:`then_1`
      (bind _asbp_third_person_character (cast `/Game/ThirdPerson/Blueprints/BP_ThirdPersonCharacter` (`GameplayStatics.GetPlayerPawn` 0)))
      (`Quest.EnableQuest` (`self.MyQuest`) (`DemoreelRPGCharacter.PlayerChannels` _asbp_third_person_character)))
    (:`then_2`
      (bind _asbp_hud (cast `/Game/MyGame/3C/_HUD/BP_HUD` (`PlayerController.GetHUD` (`GameplayStatics.GetPlayerController` 0))))
      (`KismetSystemLibrary.Delay` 0.2)
      (`/Game/MyGame/Blueprints/UI/WBP_QuestBook.AddQuest` (`/Game/MyGame/3C/_HUD/BP_HUD.QuestBookWidget` _asbp_hud) (`self.MyQuest`)))))

(event `self.ReceiveTick`
  (params (DeltaSeconds :type "Float (single-precision)"))
  ;[1 1 1] Debug purpose
  (`KismetSystemLibrary.Delay` 2.5)
  (bind _asbp_hud (cast `/Game/MyGame/3C/_HUD/BP_HUD` (`PlayerController.GetHUD` (`GameplayStatics.GetPlayerController` 0))))
  (`/Game/MyGame/Blueprints/UI/WBP_QuestBook.UpdateQuestBook` (`/Game/MyGame/3C/_HUD/BP_HUD.QuestBookWidget` _asbp_hud) (`self.MyQuest`)))

(fn `UserConstructionScript`)